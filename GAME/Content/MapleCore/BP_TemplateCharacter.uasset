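; Template player character that wires the MapleCore inventory and weapon system to player input.
; On BeginPlay the authority creates and pushes AK74 and M16 inventories, attaching the AK74 to inventory bar slot 1, while remotes call draw on that slot.
; Launch and Reload inputs enter or leave gameplay-tag outer states, and T toggles the drawn weapon's launch mode.
; Accessor functions expose the InventoryManager, first- or third-person mesh and local control.
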(event `self.ReceiveBeginPlay`
  (bind _inventorymanager (`self.InventoryManager`))
  (`/Engine/EditorBlueprintResources/ActorMacros.Switch Has Authority`
    (:`Authority`
      (`|ExecutionSequence`
        (:`then_0`
          (bind _returnvalue (`InventoryManagerBase.CreateInventory` (`self.InventoryManager`) "/Game/MapleCore/Inventory/CFGs/AK74/BP_Inventory_AK74.BP_Inventory_AK74_C"))
          (bind _output_get (set `self.TempInventory` _returnvalue))
          (`InventoryManagerBase.PushInventory` (`self.InventoryManager`) _output_get)
          (`BaseInventoryHelpers.InventoryAttach` _inventorymanager (`self.TempInventory`) (`InventoryManager.GetInventoryBar` _inventorymanager) 1))
        (:`then_1`
          (bind _returnvalue_2 (`InventoryManagerBase.CreateInventory` (`self.InventoryManager`) "/Game/MapleCore/Inventory/CFGs/M16/BP_Inventory_M16.BP_Inventory_M16_C"))
          (`InventoryManagerBase.PushInventory` (`self.InventoryManager`) _returnvalue_2))))
    (:`Remote`
      (`InventoryHelpers.DrawInventory` (`self.InventoryManager`) 1))))

(event `InputAction|Launch`
  (params (Key :type "Key Structure"))
  (:`Pressed`
    (`InventoryManager.EnterOuterState` (`self.InventoryManager`) (`BlueprintGameplayTagLibrary.MakeLiteralGameplayTag` (struct :`TagName` "WeaponOuterState.WantsToLaunch"))))
  (:`Released`
    (`InventoryManager.LeaveOuterState` (`self.InventoryManager`) (`BlueprintGameplayTagLibrary.MakeLiteralGameplayTag` (struct :`TagName` "WeaponOuterState.WantsToLaunch")))))

(event `InputAction|Reload`
  (params (Key :type "Key Structure"))
  (:`Pressed`
    (`InventoryManager.EnterOuterState` (`self.InventoryManager`) (`BlueprintGameplayTagLibrary.MakeLiteralGameplayTag` (struct :`TagName` "WeaponOuterState.WantsToReload"))))
  (:`Released`
    (`InventoryManager.LeaveOuterState` (`self.InventoryManager`) (`BlueprintGameplayTagLibrary.MakeLiteralGameplayTag` (struct :`TagName` "WeaponOuterState.WantsToReload")))))

(event `Key|T`
  (params (Key :type "Key Structure"))
  (:`Pressed`
    (`self.ToggleWeaponLaunchMode`)))

(event `Key|NumPadZero`
  (params (Key :type "Key Structure")))

(event `Key|NumPadOne`
  (params (Key :type "Key Structure")))

(event `Key|NumPadTwo`
  (params (Key :type "Key Structure")))

(event `Key|NumPadThree`
  (params (Key :type "Key Structure")))

(event `Key|NumPadFour`
  (params (Key :type "Key Structure")))

(event `Key|NumPadFive`
  (params (Key :type "Key Structure")))

(event `Key|Subtract`
  (params (Key :type "Key Structure")))

(event `Key|Add`
  (params (Key :type "Key Structure")))

(fn `GetInventoryManager`
  (returns (ReturnValue :type "InventoryManagerBase Object Reference"))
  (bind _returnvalue (`self.GetInventoryManager_BP`))
  (return _returnvalue))

(fn `GetInventoryManager_BP`
  (returns (ReturnValue :type "InventoryManagerBase Object Reference"))
  (return (`self.InventoryManager`)))

(fn `GetOwnerMesh`
  (params (bIsFPP :type Boolean))
  (returns (ReturnValue :type "SkeletalMeshComponent Object Reference"))
  (bind _returnvalue (`self.GetOwnerMesh_BP` bIsFPP))
  (return _returnvalue))

(fn `GetOwnerMesh_BP`
  (params (bIsFPP :type Boolean :default false))
  (returns (ReturnValue :type "SkeletalMeshComponent Object Reference"))
  (return (select `bool` bIsFPP :`false` (`self.Mesh`) :`true` (`self.Mesh1p`))))

(fn `IsLocallyOwned`
  (returns (ReturnValue :type Boolean))
  (bind _returnvalue (`self.IsLocallyOwned_BP`))
  (return _returnvalue))

(fn `IsLocallyOwned_BP`
  (returns (ReturnValue :type Boolean))
  (return (`self.IsLocallyControlled`)))

(fn `ToggleWeaponLaunchMode`
  (bind _returnvalue (`InventoryManager.GetDrawnInventory` (`self.InventoryManager`)))
  (bind _returnvalue_2 (`Inventory.GetInventoryActor` _returnvalue))
  (bind _returnvalue_3 (`self.GetComponentByClass` _returnvalue_2 "/Script/GAME.WeaponLaunchSystem"))
  (`/Engine/EditorBlueprintResources/StandardMacros.IsValid` _returnvalue
    (:`Is Valid`
      (`/Engine/EditorBlueprintResources/StandardMacros.IsValid` _returnvalue_2
        (:`Is Valid`
          (`/Engine/EditorBlueprintResources/StandardMacros.IsValid` _returnvalue_3
            (:`Is Valid`
              (`WeaponLaunchSystem.ToggleLaunchMode` _returnvalue_3))))))))

(fn `UserConstructionScript`)