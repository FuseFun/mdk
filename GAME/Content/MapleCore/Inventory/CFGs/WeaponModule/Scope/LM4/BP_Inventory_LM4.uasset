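; Inventory item for the LM4 scope weapon module, managing the scope's static mesh through inventory lifecycle events.
; Enter spawns a hidden, collision-free mesh component on the owner and leave destroys it.
; Attach caches the socket name from the parent inventory place, draw snaps the mesh onto the parent item's first-person component, and show/unshow toggle visibility.
; It also exposes its own mesh as the first-person attach component.
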(event `self.K2_OnEnter`
  (`self.Mesh`
    (:`then`)
    (:`else`
      (bind _output_get (set `self.Owner` (`self.GetOwner`)))
      (`/Engine/EditorBlueprintResources/StandardMacros.IsValid` _output_get
        (:`Is Valid`
          (bind _returnvalue (`|AddComponentByClass` (`self.Owner`) "/Script/Engine.StaticMeshComponent" true (`self.Zero Transform`)))
          (`/Engine/EditorBlueprintResources/StandardMacros.IsValid` _returnvalue
            (:`Is Valid`
              (bind _output_get_2 (set `self.Mesh` _returnvalue))
              (`PrimitiveComponent.SetCollisionEnabled` _output_get_2 "NoCollision")
              (`StaticMeshComponent.SetStaticMesh` _output_get_2 "/Game/Assets/CZ_LM4/SM_CZ_LM4.SM_CZ_LM4")
              (`SceneComponent.SetVisibility` _output_get_2 false false))))))))

(event `self.K2_OnLeave`
  (`self.Mesh`
    (:`then`
      (`ActorComponent.K2_DestroyComponent` (`self.Mesh`)))
    (:`else`
      _))
  (set `self.Owner` null))

(event `self.K2_OnDraw`
  (params (Inventory :type "Inventory Object Reference") (bAttach :type Boolean))
  (bind _returnvalue (`self.GetFatherInventory`))
  (`/Engine/EditorBlueprintResources/StandardMacros.IsValid` (`self.GetInventoryActor` Inventory)
    (:`Is Valid`
      (`/Engine/EditorBlueprintResources/StandardMacros.IsValid` _returnvalue
        (:`Is Valid`
          (bind _output_get (set `self.FatherInventory` _returnvalue))
          (bind _output_get_2 (set `self.Default Attach Comp` (`self.GetDefaultAttachComponentCustom` _output_get true)))
          (`/Engine/EditorBlueprintResources/StandardMacros.IsValid` _output_get_2
            (:`Is Valid`
              (bind _mesh (`self.Mesh`)
                (:`then`
                  (bind _returnvalue_2 (`SceneComponent.K2_AttachToComponent` _mesh (`self.Default Attach Comp`) (`self.AttachTo`) "KeepRelative" "KeepRelative" "KeepRelative" true))
                  (if _returnvalue_2
                    (`SceneComponent.K2_SetRelativeTransform` (`self.Mesh`) (`self.Zero Transform`) false false)))
                (:`else`)))))))))

(event `self.K2_OnUndraw`
  (params (Inventory :type "Inventory Object Reference") (bDetach :type Boolean))
  (`/Engine/EditorBlueprintResources/StandardMacros.IsValid` (`self.Mesh`)
    (:`Is Valid`
      (`SceneComponent.K2_DetachFromComponent` (`self.Mesh`) "KeepWorld" "KeepWorld" "KeepWorld" true))))

(event `self.K2_OnShow`
  (bind _mesh (`self.Mesh`)
    (:`then`
      (`SceneComponent.SetVisibility` _mesh true false))
    (:`else`)))

(event `self.K2_OnUnshow`
  (bind _mesh (`self.Mesh`)
    (:`then`
      (`SceneComponent.SetVisibility` _mesh false false))
    (:`else`)))

(event `self.K2_OnAttach`
  (bind _returnvalue (`self.GetFatherInventoryPlace`))
  (`/Engine/EditorBlueprintResources/StandardMacros.IsValid` _returnvalue
    (:`Is Valid`
      (set `self.AttachTo` (`InventoryPlace.GetAttachSocketName` _returnvalue (`self.Category`))))))

(fn `GetDefaultAttachComponentCustom`
  (params (bIsFPP :type Boolean))
  (returns (ReturnValue :type "SceneComponent Object Reference"))
  (return (select `bool` bIsFPP :`true` (`self.Mesh`) :!type "SceneComponent Object Reference")))