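; Inventory weapon module for the M16 base iron sight, showing the carry handle mesh on the parent weapon.
; On attach it gets the socket name for its category from the parent's inventory place.
; On draw it creates a collision-free static mesh component on the parent's first-person attach component; show, unshow and undraw toggle or destroy it.
; It exposes that mesh as the first-person attach component for child attachments.
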(event `self.K2_OnDraw`
  (params (Inventory :type "Inventory Object Reference") (bAttach :type Boolean))
  (bind _returnvalue (`self.GetInventoryActor` Inventory))
  (bind _returnvalue_2 (`self.GetFatherInventory`))
  (bind _returnvalue_3 (`self.GetDefaultAttachComponentCustom` _returnvalue_2 true))
  (`/Engine/EditorBlueprintResources/StandardMacros.IsValid` _returnvalue
    (:`Is Valid`
      (`/Engine/EditorBlueprintResources/StandardMacros.IsValid` _returnvalue_2
        (:`Is Valid`
          (`/Engine/EditorBlueprintResources/StandardMacros.IsValid` _returnvalue_3
            (:`Is Valid`
              (bind _returnvalue_4 (`|AddComponentByClass` _returnvalue "/Script/Engine.StaticMeshComponent" true (`self.Zero Transform`)))
              (`/Engine/EditorBlueprintResources/StandardMacros.IsValid` _returnvalue_4
                (:`Is Valid`
                  (bind _output_get (set `self.Mesh` _returnvalue_4))
                  (bind _returnvalue_5 (`SceneComponent.K2_AttachToComponent` _output_get _returnvalue_3 (`self.AttachTo`) "KeepRelative" "KeepRelative" "KeepRelative" true))
                  (if _returnvalue_5
                    (`SceneComponent.K2_SetRelativeTransform` (`self.Mesh`) (`self.Zero Transform`) false false)
                    (`PrimitiveComponent.SetCollisionEnabled` (`self.Mesh`) "NoCollision")
                    (`StaticMeshComponent.SetStaticMesh` (`self.Mesh`) "/Game/Assets/Weapons_A001/Meshes/M16/SM_M16_CarryHandle.SM_M16_CarryHandle")))))))))))

(event `self.K2_OnUndraw`
  (params (Inventory :type "Inventory Object Reference") (bDetach :type Boolean))
  (`/Engine/EditorBlueprintResources/StandardMacros.IsValid` (`self.Mesh`)
    (:`Is Valid`
      (`ActorComponent.K2_DestroyComponent` (`self.Mesh`))
      (set `self.Mesh` null))))

(event `self.K2_OnShow`
  (bind _mesh (`self.Mesh`)
    (:`then`
      (`SceneComponent.SetVisibility` _mesh true false))
    (:`else`)))

(event `self.K2_OnUnshow`
  (bind _mesh (`self.Mesh`)
    (:`then`
      (`SceneComponent.SetVisibility` _mesh false false))
    (:`else`)))

(event `self.K2_OnAttach`
  (bind _returnvalue (`self.GetFatherInventoryPlace`))
  (`/Engine/EditorBlueprintResources/StandardMacros.IsValid` _returnvalue
    (:`Is Valid`
      (set `self.AttachTo` (`InventoryPlace.GetAttachSocketName` _returnvalue (`self.Category`))))))

(fn `GetDefaultAttachComponentCustom`
  (params (bIsFPP :type Boolean))
  (returns (ReturnValue :type "SceneComponent Object Reference"))
  (return (select `bool` bIsFPP :`true` (`self.Mesh`) :!type "SceneComponent Object Reference")))