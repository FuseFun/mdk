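; M16 base iron sight inventory item that shows the carry handle mesh on its parent item.
; On attach it caches the socket name for its category from the parent inventory bar's CDO.
; Drawing spawns a collision-free static mesh component on the inventory actor at that socket, undraw destroys it, and show or unshow toggles visibility.
; GetAttachROOT returns this mesh as the first-person attach root.
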(event `self.K2_OnDraw`
  (params (Inventory :type "Inventory Object Reference") (bAttach :type Boolean))
  (bind _returnvalue (`self.GetInventoryActor` Inventory))
  (`/Engine/EditorBlueprintResources/StandardMacros.IsValid` _returnvalue
    (:`Is Valid`
      (bind _asinventory (cast `Inventory` (`self.GetFatherInventory`)))
      (bind _returnvalue_2 (`self.GetAttachROOT` _asinventory true))
      (`/Engine/EditorBlueprintResources/StandardMacros.IsValid` _returnvalue_2
        (:`Is Valid`
          (bind _returnvalue_3 (`|AddComponentByClass` _returnvalue "/Script/Engine.StaticMeshComponent" true (`self.Zero Transform`)))
          (`/Engine/EditorBlueprintResources/StandardMacros.IsValid` _returnvalue_3
            (:`Is Valid`
              (bind _output_get (set `self.Mesh` _returnvalue_3))
              (bind _returnvalue_4 (`SceneComponent.K2_AttachToComponent` _output_get _returnvalue_2 (`self.AttachTo`) "KeepRelative" "KeepRelative" "KeepRelative" true))
              (if _returnvalue_4
                (`SceneComponent.K2_SetRelativeTransform` (`self.Mesh`) (`self.Zero Transform`) false false)
                (`PrimitiveComponent.SetCollisionEnabled` (`self.Mesh`) "NoCollision")
                (`StaticMeshComponent.SetStaticMesh` (`self.Mesh`) "/Game/Assets/Weapons_A001/Meshes/M16/SM_M16_CarryHandle.SM_M16_CarryHandle")))))))))

(event `self.K2_OnUndraw`
  (params (Inventory :type "Inventory Object Reference") (bDetach :type Boolean))
  (`/Engine/EditorBlueprintResources/StandardMacros.IsValid` (`self.Mesh`)
    (:`Is Valid`
      (`ActorComponent.K2_DestroyComponent` (`self.Mesh`))
      (set `self.Mesh` null))))

(event `self.K2_OnShow`
  (bind _mesh (`self.Mesh`)
    (:`then`
      (`SceneComponent.SetVisibility` _mesh true false))
    (:`else`)))

(event `self.K2_OnUnshow`
  (bind _mesh (`self.Mesh`)
    (:`then`
      (`SceneComponent.SetVisibility` _mesh false false))
    (:`else`)))

(event `self.K2_OnAttach`
  (bind _asinventory_bar (cast `InventoryBar` (`self.GetFatherInventoryBarCDO`)))
  (set `self.AttachTo` (`InventoryBar.GetAttachSocketName` _asinventory_bar (`self.Category`))))

(fn `GetAttachROOT`
  (params (bIsFPP :type Boolean))
  (returns (ReturnValue :type "SceneComponent Object Reference"))
  (return (select `bool` bIsFPP :`true` (`self.Mesh`) :!type "SceneComponent Object Reference")))