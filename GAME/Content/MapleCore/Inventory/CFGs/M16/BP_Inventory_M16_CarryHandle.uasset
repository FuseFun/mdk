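; Inventory config for the M16 carry handle attachment, adding its static mesh to the weapon's inventory actor.
; On draw it creates a static mesh component at runtime, attaches it to the actor mesh's RailSocket and disables its collision.
; Undraw destroys that component, while show and unshow toggle its visibility.
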(event `self.OnDraw_Custom`
  (params (Inventory :type "Inventory Object Reference") (bAttach :type Boolean))
  (bind _returnvalue (`self.GetInventoryActor` Inventory))
  (bind _returnvalue_2 (`InventoryActor.GetMesh` _returnvalue true))
  (`/Engine/EditorBlueprintResources/StandardMacros.IsValid` _returnvalue
    (:`Is Valid`
      (`/Engine/EditorBlueprintResources/StandardMacros.IsValid` _returnvalue_2
        (:`Is Valid`
          (bind _returnvalue_3 (`|AddComponentByClass` _returnvalue "/Script/Engine.StaticMeshComponent" true (`self.Zero Transform`)))
          (`/Engine/EditorBlueprintResources/StandardMacros.IsValid` _returnvalue_3
            (:`Is Valid`
              (bind _output_get (set `self.Mesh` _returnvalue_3))
              (bind _returnvalue_4 (`SceneComponent.K2_AttachToComponent` _output_get _returnvalue_2 "RailSocket" "KeepRelative" "KeepRelative" "KeepRelative" true))
              (if _returnvalue_4
                (`SceneComponent.K2_SetRelativeTransform` (`self.Mesh`) (`self.Zero Transform`) false false)
                (`PrimitiveComponent.SetCollisionEnabled` (`self.Mesh`) "NoCollision")
                (`StaticMeshComponent.SetStaticMesh` (`self.Mesh`) "/Game/Assets/Weapons_A001/Meshes/M16/SM_M16_CarryHandle.SM_M16_CarryHandle")))))))))

(event `self.OnUndraw_Custom`
  (params (Inventory :type "Inventory Object Reference") (bDetach :type Boolean))
  (`/Engine/EditorBlueprintResources/StandardMacros.IsValid` (`self.Mesh`)
    (:`Is Valid`
      (`ActorComponent.K2_DestroyComponent` (`self.Mesh`))
      (set `self.Mesh` null))))

(event `self.OnShow_Custom`
  (bind _mesh (`self.Mesh`)
    (:`then`
      (`SceneComponent.SetVisibility` _mesh true false))
    (:`else`)))

(event `self.OnUnshow_Custom`
  (bind _mesh (`self.Mesh`)
    (:`then`
      (`SceneComponent.SetVisibility` _mesh false false))
    (:`else`)))