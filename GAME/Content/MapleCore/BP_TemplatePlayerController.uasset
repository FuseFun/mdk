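; Template player controller for MapleCore that drives the inventory page and inventory drawing, with built-in debug aids.
; Key E lazily creates, binds and shows the inventory page through the UI manager; number keys draw inventory slots.
; BeginPlay shows a logo and applies display settings locally, and simulates heavy packet lag on remote clients.
; Tick prints held and drawn inventories, colored by authority, and an event destroys the controlled pawn.
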(event `self.ReceiveBeginPlay`
  (`|ExecutionSequence`
    (:`then_0`
      (`/Engine/EditorBlueprintResources/ActorMacros.Switch Has Authority`
        (:`Remote`
          (`KismetSystemLibrary.ExecuteConsoleCommand` "Net PktLag=1000" self)
          (`KismetSystemLibrary.ExecuteConsoleCommand` "Net PktLagVariance=500" self))))
    (:`then_1`
      (if (`self.IsLocalPlayerController`)
        (`self.ShowLogo`)
        (`KismetSystemLibrary.ExecuteConsoleCommand` "t.MaxFPS 0" self)
        (`KismetSystemLibrary.ExecuteConsoleCommand` "r.VSync 1" self)
        (`KismetSystemLibrary.ExecuteConsoleCommand` "r.MotionBlur.Scale 0.5" self)))))

(event `Key|E`
  (params (Key :type "Key Structure"))
  (:`Pressed`
    (bind _output_get (set `self.InventoryManager` (`InventoryHelpers.GetInventoryManager` (`/Game/MapleCore/Inventory/BPFL_InventoryHelpers.GetInventoryHolder`))))
    (`/Engine/EditorBlueprintResources/StandardMacros.IsValid` _output_get
      (:`Is Valid`
        (`self.InventoryPageUMG`
          (:`then`
            _)
          (:`else`
            (bind _returnvalue (`|CreateWidget` "/Game/MapleCore/Inventory/UMG_Page_Inventory.UMG_Page_Inventory_C" self))
            (bind _output_get_2 (set `self.InventoryPageUMG` _returnvalue))
            (`/Engine/EditorBlueprintResources/StandardMacros.IsValid` _output_get_2
              (:`Is Valid`
                (`InventoryManagerBase.BindInventoryInterface` (`self.InventoryManager`) (`self.InventoryPageUMG`))))))
        (`UserInterfaceManager.AddToManager` (`self.UserInterfaceManager`) (`self.InventoryPageUMG`))))))

(event `Key|One`
  (params (Key :type "Key Structure"))
  (:`Pressed`
    (`InventoryHelpers.DrawInventory` (`InventoryHelpers.GetInventoryManager` (`/Game/MapleCore/Inventory/BPFL_InventoryHelpers.GetInventoryHolder`)) 1)))

(event `Key|Two`
  (params (Key :type "Key Structure"))
  (:`Pressed`
    (`InventoryHelpers.DrawInventory` (`InventoryHelpers.GetInventoryManager` (`/Game/MapleCore/Inventory/BPFL_InventoryHelpers.GetInventoryHolder`)) 2)))

(event `self.ReceiveTick`
  (params (DeltaSeconds :type "Float (single-precision)"))
  (`|ExecutionSequence`
    (:`then_0`
      (`self.LogInventory`))))

(event `ServerDestroyPawn`
  (`self.K2_DestroyActor` (`self.K2_GetPawn`)))

(fn `DebugA`
  (`KismetSystemLibrary.PrintString` "DebugA" false true (struct :`G` 0.66 :`B` 1.0 :`A` 1.0) 0.0)
  (`self.ServerDestroyPawn`))

(fn `LogInventory`
  (locals (MyInventoryManager :type "InventoryManager Object Reference") (IsDrawn :type Boolean :default false))
  (bind _myinventorymanager (`local.MyInventoryManager`))
  (bind _myinventorymanager_2 (`local.MyInventoryManager`))
  (bind _returnvalue (`InventoryManager.GetDrawnInventory` _myinventorymanager_2))
  (bind _output_get (set `local.MyInventoryManager` (`InventoryHelpers.GetInventoryManager` (`/Game/MapleCore/Inventory/BPFL_InventoryHelpers.GetInventoryHolder`))))
  (`/Engine/EditorBlueprintResources/StandardMacros.IsValid` _output_get
    (:`Is Valid`
      (`|ExecutionSequence`
        (:`then_0`
          (`/Engine/EditorBlueprintResources/StandardMacros.IsValid` _myinventorymanager
            (:`Is Valid`
              (bind _values (`BlueprintMapLibrary.Map_Values` (`InventoryManagerBase.GetInventoryMap` _myinventorymanager)))
              (for _array_element _values
                (`/Engine/EditorBlueprintResources/StandardMacros.IsValid` _array_element
                  (:`Is Valid`
                    (`KismetSystemLibrary.PrintText` (`|FormatText` "InventoryName= {0}" (`InventoryBase.GetInventoryName` _array_element)) true false (select `bool` (`self.HasAuthority`) :`false` (struct :`G` 1.0 :`A` 1.0) :`true` (struct :`R` 1.0 :`A` 1.0) :!type "LinearColor Structure") 0.0)))))))
        (:`then_1`
          (`/Engine/EditorBlueprintResources/StandardMacros.IsValid` _returnvalue
            (:`Is Valid`
              (`KismetSystemLibrary.PrintText` (`|FormatText` "[{0}] Drawn Inventory= {1}" (`InventoryManager.GetDrawnInventoryPlaceID` _myinventorymanager_2) (`InventoryBase.GetInventoryName` _returnvalue)) true false (select `bool` (`self.HasAuthority`) :`false` (struct :`G` 1.0 :`A` 1.0) :`true` (struct :`R` 1.0 :`A` 1.0) :!type "LinearColor Structure") 0.0))))))))

(fn `ShowLogo`
  (bind _returnvalue (`|CreateWidget` "/Game/MapleCore/Logo/UMG_Logo.UMG_Logo_C" self))
  (`UserWidget.AddToViewport` _returnvalue 0))

(fn `UserConstructionScript`)